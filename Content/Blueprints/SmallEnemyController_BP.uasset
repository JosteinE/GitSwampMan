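; SmallEnemyController_BP drives a small enemy that fires bullets automatically at a fixed interval.
; BeginPlay starts a looping named timer and caches the player pawn, cast to MyPlayerCharacterWithCamera_BP, though nothing here uses that reference.
; Each FireRate tick spawns an EnemyBullet just ahead of the actor along its current facing, with no aiming at the player.
; Overlap, Tick and Hit events are empty.
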(event Custom|FireRate
  (bind _returnvalue (Transformation|GetActorRotation))
  ;[1 1 1] Handle Firing
  (Game|SpawnActorfromClass "/Game/Blueprints/EnemyBullet.EnemyBullet_C" (Math|Transform|MakeTransform (+ (Transformation|GetActorLocation) (* (Math|Vector|GetForwardVector _returnvalue) 8e+01)) _returnvalue) "Undefined" 0 0))

(event EventBeginPlay
  ;[1 1 1] Handle Firing
  (Utilities|Time|SetTimerbyFunctionName 0 "FireRate" 2.5 true)
  (bind _asmy_player_character_with_camera_bp (Utilities|Casting|CastToMyPlayerCharacterWithCamera_BP (Game|Player|GetPlayerPawn 0)))
  (Variables|Default|SetPlayer _asmy_player_character_with_camera_bp))

(event Collision|EventActorBeginOverlap
  (params (OtherActor :type Actor%20Object%20Reference)))

(event EventTick
  (params (DeltaSeconds :type Float%20%28single-precision%29)))

(event Collision|EventHit
  (params (MyComp :type Primitive%20Component%20Object%20Reference) (Other :type Actor%20Object%20Reference) (OtherComp :type Primitive%20Component%20Object%20Reference) (bSelfMoved :type Boolean) (HitLocation :type Vector :default "0, 0, 0") (HitNormal :type Vector :default "0, 0, 0") (NormalImpulse :type Vector :default "0, 0, 0") (Hit :type Hit%20Result%20Structure%20%28by%20ref%29))
  ;[1 1 1] On Hit
)

(fn ConstructionScript)